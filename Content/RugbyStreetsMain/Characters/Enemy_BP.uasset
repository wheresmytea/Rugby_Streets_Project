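; Enemy character Blueprint that notices the player when they carry the ball.
; PawnSensing's OnSeePawn casts the seen pawn to player_BP and, if CarryingBall is true, sets the hasSeenPlayer Blackboard bool on its AI controller.
; An AIPerception update event is bound but empty, with its debug print and player cast left disconnected.
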(event `self.PawnSensing.OnSeePawn`
  (params (Pawn :type "Pawn Object Reference"))
  (bind _asplayer_bp (cast `/Game/RugbyStreetsMain/Characters/player_BP` Pawn))
  (if (`/Game/RugbyStreetsMain/Characters/player_BP.carryingBall` _asplayer_bp)
    (`BlackboardComponent.SetValueAsBool` (`AIBlueprintHelperLibrary.GetBlackboard` (`AIBlueprintHelperLibrary.GetAIController` self)) "hasSeenPlayer" true)))

(event `self.AIPerception.OnPerceptionUpdated`
  (params (UpdatedActors :type "Array of Actor Object Reference (by ref)")))

(fn `UserConstructionScript`)